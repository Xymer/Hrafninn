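; BP_Chandelier is a realm-switching scene chandelier built to swing and optionally spin, using two timelines.
; The construction script sets swing direction and rate, and plays or stops RotationTimer based on the Rotate flag.
; RotationTimer yaws the skeletal mesh by a range re-randomized every few seconds, while SwingTimer rolls the actor around the mesh's starting rotation.
; No graph wire starts SwingTimer.
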(event Custom|SetRandomRotation
  (Variables|Default|SetRandomRange (Math|Random|RandomFloatinRange 45.0 6e+01)))

(event EventBeginPlay
  (Variables|Default|SetRotationOrigin (Transformation|GetWorldRotation (Variables|Default|GetSkeletalMesh)))
  (Utilities|Time|SetTimerbyEvent (delegate Custom|SetRandomRotation) 5.0 true))

(fn ConstructionScript
  (bind _rotationtimer (Variables|Default|GetRotationTimer))
  (bind _swingamount (Variables|Default|GetSwingAmount))
  (Utilities|FlowControl|Sequence
    (:then_0
      (Variables|Default|SetXRotation (Math|Float|SelectFloat (* _swingamount -1.0) _swingamount (Variables|Default|GetSwingClockwise?))))
    (:then_1
      (Components|Timeline|SetPlayRate (Variables|Default|GetSwingTimer) (Variables|Default|GetSwingRate)))
    (:then_2
      (if (Variables|Default|GetRotate?)
        (Audio|Components|Audio|Play _rotationtimer)
        (else
          (Audio|Components|Audio|Stop _rotationtimer))))))