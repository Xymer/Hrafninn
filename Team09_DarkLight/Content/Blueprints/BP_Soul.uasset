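; Collectible soul that bobs via timeline, trails the character who picks it up, and is turned in at a lantern.
; Pickup disables collision, sets its place in line from held souls, scales it, dims its light and starts whisper audio.
; Tick moves it through SoulMovement toward the pawn beyond a set distance, or toward the lantern once turned in.
; Turn-in shrinks it and fades audio before destroying it.
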(event EventOnTurnin
  (params (Lantern :type Actor%20Object%20Reference))
  (bind _timetodestroy (Variables|Default|GetTimeToDestroy))
  (Variables|Default|SetLantern Lantern)
  (Variables|Default|SetIsTurnedIn true)
  (Utilities|FlowControl|Sequence
    (:then_0
      (bind _scale (Timeline|LowerTheScale PlayFromStart)
        (:Update
          (Transformation|SetActorScale3D _scale))))
    (:then_1
      (Audio|Components|Audio|FadeOut (Variables|Default|GetWhisperSound) _timetodestroy 0.0 "Linear" :!class /Script/Engine.AudioComponent)
      (Utilities|FlowControl|Delay _timetodestroy)
      (Actor|DestroyActor))
    (:then_2
      (bind _returnvalue (AddComponent|AddAudioComponent false))
      (Audio|Components|Audio|FadeOut _returnvalue _timetodestroy 0.0 "Linear" :!class /Script/Engine.AudioComponent))))

(event EventBeginPlay
  (bind _returnvalue (Transformation|GetActorLocation))
  (Variables|Default|SetStartLocation (Transformation|GetActorLocation))
  (bind _newtrack_0 (Timeline|Timeline_0 PlayFromStart)
    (:Update
      (Transformation|SetActorLocation (Math|Vector|MakeVector (.x _returnvalue) (.y _returnvalue) (.z (+ (Math|Vector|MakeVector 0.0 0.0 _newtrack_0) (Transformation|GetActorLocation)))) false false))
    (:Finished
      (if true
        (Timeline|Timeline_0 ReverseFromEnd)))))

(event EventTick
  (params (DeltaSeconds :type Float%20%28single-precision%29))
  (bind _lantern (Variables|Default|GetLantern))
  (bind _returnvalue (Utilities|SoulMovement _lantern))
  (if (Variables|Default|GetIsTurnedIn)
    (Transformation|SetActorLocation (Math|Vector|MakeVector (.x _returnvalue) (.y _returnvalue) (+ (.z _returnvalue) (Variables|Default|GetLamternTurnInOffset))) false false)
    (else
      (Utilities|FlowControl|Sequence
        (:then_0
          (bind _pawntofollow (Variables|Default|GetPawnToFollow)
            (:then
              (if (< (Variables|Default|GetDistanceBehindPawn) (Math|Vector|Distance(Vector) (Transformation|GetActorLocation) (Transformation|GetActorLocation _pawntofollow)))
                (Transformation|SetActorLocation (Utilities|SoulMovement (Variables|Default|GetPawnToFollow)) false false)))
            (:else)))))))

(event EventOnPickedUp
  (params (Pawn :type Pawn%20Object%20Reference))
  (Utilities|FlowControl|Sequence
    (:then_0
      (bind _asteam_09_dark_light_character (Utilities|Casting|CastToTeam09_DarkLightCharacter Pawn))
      (Variables|Default|SetPlaceInLine (+ (Utilities|Array|Length (Variables|/Script/Team09_DarkLight.Team09_DarkLightCharacter|GetHeldSouls _asteam_09_dark_light_character)) 1))
      (Variables|Default|SetPawnToFollow _asteam_09_dark_light_character)
      (Actor|Tick|SetActorTickEnabled true)
      (Collision|SetCollisionEnabled (Variables|Default|GetBoxComponent) "NoCollision")
      (Collision|SetCollisionEnabled (Variables|Default|GetBoxComponent) "NoCollision")
      (Variables|Default|SetIsTurnedIn false)
      (Class|LightComponent|SetIESBrightnessScale (Variables|Default|GetPointLight) 0.4)
      (Variables|Default|SetOriginScale (Transformation|GetActorScale3D))
      (bind _alpha (Timeline|ScaleFeedback Play)
        (:Update
          (Transformation|SetActorScale3D (Math|Vector|Lerp(Vector) (Variables|Default|GetOriginScale) (* (Variables|Default|GetOriginScale) 1.5) _alpha)))))
    (:then_1
      (bind _returnvalue (AddComponent|AddAudioComponent false))
      (Variables|Default|SetWhisperSound _returnvalue))))

(fn ConstructionScript)