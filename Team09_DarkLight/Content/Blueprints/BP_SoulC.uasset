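; Collectible soul that trails the Dark Light character once picked up and is turned in at a lantern.
; Player overlap or OnPickedUp sets its place behind HeldSouls, disables collision and adjusts the light, with overlap also calling SetUp on ASoulFollowTarget.
; Turn-in notifies that target, moves the soul via SoulMovement with a height offset, and plays a scale timeline before delayed destruction.
; Older bobbing and follow logic is disconnected.
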(event OnComponentBeginOverlap(BoxComponent)
  (params (OverlappedComponent :type Primitive%20Component%20Object%20Reference) (OtherActor :type Actor%20Object%20Reference) (OtherComp :type Primitive%20Component%20Object%20Reference) (OtherBodyIndex :type Integer) (bFromSweep :type Boolean) (SweepResult :type Hit%20Result%20Structure%20%28by%20ref%29))
  ;[1 0.09139 0] Thing2
  (if (== OtherActor (Game|Player|GetPlayerPawn 0))
    (Class|ASoulFollowTargetComponent|SetUp (Variables|Default|GetASoulFollowTarget) (Variables|Default|GetPawnToFollow))
    (bind _asteam_09_dark_light_character (Utilities|Casting|CastToTeam09_DarkLightCharacter (stale EventOnPickedUp Pawn)))
    (Variables|Default|SetPlaceInLine (+ (Utilities|Array|Length (Variables|/Script/Team09_DarkLight.Team09_DarkLightCharacter|GetHeldSouls _asteam_09_dark_light_character)) 1))
    (Variables|Default|SetPawnToFollow _asteam_09_dark_light_character)
    (Actor|Tick|SetActorTickEnabled true)
    (Collision|SetCollisionEnabled (Variables|Default|GetBoxComponent) "NoCollision")
    (Collision|SetCollisionEnabled (Variables|Default|GetBoxComponent) "NoCollision")
    (Variables|Default|SetIsTurnedIn false)
    (Class|LightComponent|SetIESBrightnessScale (Variables|Default|GetPointLight) 0.4)))

(event EventOnTurnin
  (params (Lantern :type Actor%20Object%20Reference))
  (bind _timetodestroy (Variables|Default|GetTimeToDestroy))
  ;[0.1084 1 0] Thing4
  (bind _output_get (Variables|Default|SetLantern Lantern))
  (Class|ASoulFollowTargetComponent|SoulTurnedin (Variables|Default|GetASoulFollowTarget) _output_get)
  (Variables|Default|SetIsTurnedIn true)
  (bind _scale (Timeline|LowerTheScale PlayFromStart)
    (:Update
      (Transformation|SetActorScale3D _scale)
      (Utilities|FlowControl|Delay _timetodestroy)
      (Actor|DestroyActor))))

(event EventBeginPlay
  ;[1 0 0.04811] Thing1
)

(event EventTick
  (params (DeltaSeconds :type Float%20%28single-precision%29))
  (bind _lantern (Variables|Default|GetLantern))
  (bind _returnvalue (Utilities|SoulMovement _lantern))
  ;[1 0.8366 0] Thing3
  (if (Variables|Default|GetIsTurnedIn)
    (Transformation|SetActorLocation (Math|Vector|MakeVector (.x _returnvalue) (.y _returnvalue) (+ (.z _returnvalue) (Variables|Default|GetLamternTurnInOffset))) false false)))

(event EventOnPickedUp
  (params (Pawn :type Pawn%20Object%20Reference))
  ;[1 0.09139 0] Thing2
  (bind _asteam_09_dark_light_character (Utilities|Casting|CastToTeam09_DarkLightCharacter Pawn))
  (Variables|Default|SetPlaceInLine (+ (Utilities|Array|Length (Variables|/Script/Team09_DarkLight.Team09_DarkLightCharacter|GetHeldSouls _asteam_09_dark_light_character)) 1))
  (Variables|Default|SetPawnToFollow _asteam_09_dark_light_character)
  (Actor|Tick|SetActorTickEnabled true)
  (Collision|SetCollisionEnabled (Variables|Default|GetBoxComponent) "NoCollision")
  (Collision|SetCollisionEnabled (Variables|Default|GetBoxComponent) "NoCollision")
  (Variables|Default|SetIsTurnedIn false)
  (Class|LightComponent|SetIESBrightnessScale (Variables|Default|GetPointLight) 0.4))

(fn ConstructionScript)