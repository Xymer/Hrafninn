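; BP_Mast is a realm-reactive mast object that changes its look and behavior when the world swaps between Dark and Light realms.
; Its OnSwapRealm event swaps the Cube component's mesh to match the current realm.
; In Dark it becomes grabbable and simulates physics, while in Light it is non-grabbable with physics simulation off.
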(event EventBeginPlay
  (|CallParentFunction) ; This node is disabled and will not be called.\nDrag off pins to build functionality.
)

(event Collision|EventActorBeginOverlap
  (params (OtherActor :type Actor%20Object%20Reference))
  (|CallParentFunction OtherActor) ; This node is disabled and will not be called.\nDrag off pins to build functionality.
)

(event EventTick
  (params (DeltaSeconds :type Float%20%28single-precision%29))
  (|CallParentFunction DeltaSeconds) ; This node is disabled and will not be called.\nDrag off pins to build functionality.
)

(event EventOnSwapRealm
  (params (CurrentRealm :type RealmType%20Enum :default "Dark"))
  (switch Utilities|FlowControl|Switch|SwitchonRealmType CurrentRealm
    (:Dark
      (Variables|Default|SetbIsGrabbable true)
      (Components|StaticMesh|SetStaticMesh (Variables|Default|GetCube) (Variables|Default|GetDarkMesh))
      (Physics|SetSimulatePhysics (Variables|Default|GetCube) true))
    (:Light
      (Variables|Default|SetbIsGrabbable false)
      (Components|StaticMesh|SetStaticMesh (Variables|Default|GetCube) (Variables|Default|GetLightMesh))
      (Physics|SetSimulatePhysics (Variables|Default|GetCube) false))))

(fn ConstructionScript
  (|CallParentFunction))