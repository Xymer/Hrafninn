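; BP_LevelTransition is a trigger actor that fades the screen and loads a level when the player enters its box.
; On BeginPlay it creates a TransitionFade widget and, after a short delay, runs the FadeIn timeline on its BlackScreen opacity.
; The first box overlap sets a one-shot flag before the player check.
; A player overlap then plays FadeOut, waits briefly and calls LoadLevel on ALevelList.
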(event OnComponentBeginOverlap(Box)
  (params (OverlappedComponent :type Primitive%20Component%20Object%20Reference) (OtherActor :type Actor%20Object%20Reference) (OtherComp :type Primitive%20Component%20Object%20Reference) (OtherBodyIndex :type Integer) (bFromSweep :type Boolean) (SweepResult :type Hit%20Result%20Structure%20%28by%20ref%29))
  (if (not (Variables|Default|GetisTriggerd))
    (Variables|Default|SetisTriggerd true)
    (if (== OtherActor (Game|Player|GetPlayerPawn 0))
      (bind _fadeouttrack (Timeline|FadeOut PlayFromStart)
        (:Update
          (Widget|SetRenderOpacity (Variables|/Game/Blueprints/Widgets/LevelTransition/TransitionFade.TransitionFade_C|GetBlackScreen (Variables|Default|GetWidget)) _fadeouttrack))
        (:Finished
          (Utilities|FlowControl|Delay 1.0)
          (Class|ALevelList|LoadLevel (Variables|Default|GetALevelList)))))))

(event EventBeginPlay
  (bind _returnvalue (UserInterface|CreateWidget "/Game/Blueprints/Widgets/LevelTransition/TransitionFade.TransitionFade_C"))
  (UserInterface|Viewport|AddtoViewport _returnvalue 0)
  (Variables|Default|SetWidget _returnvalue)
  (Utilities|FlowControl|Delay 1.0)
  (bind _fadeintrack (Timeline|FadeIn PlayFromStart)
    (:Update
      (Widget|SetRenderOpacity (Variables|/Game/Blueprints/Widgets/LevelTransition/TransitionFade.TransitionFade_C|GetBlackScreen (Variables|Default|GetWidget)) _fadeintrack))))

(fn ConstructionScript)