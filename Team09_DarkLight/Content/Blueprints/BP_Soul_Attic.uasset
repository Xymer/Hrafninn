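; Collectible soul that bobs on a timeline, trails the player once picked up, and is turned in at a lantern.
; Pickup records its place among held souls, scales it up, brightens its lights and enables tick-driven following.
; It chains random whisper sounds, intended to avoid immediate repeats.
; Turn-in moves it toward the lantern, notifies Telie through LastSoulTurnedIn, then shrinks, fades audio and destroys it, with force feedback.
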(event Custom|OnAudioFinished_Event_0
  (bind _whispersounds (Variables|Default|GetWhisperSounds))
  (bind _returnvalue (Utilities|Array|Length _whispersounds))
  (bind _returnvalue_2 (- _returnvalue 1))
  (bind _returnvalue_3 (Math|Random|RandomInteger _returnvalue_2))
  (bind _output (Utilities|Array|Get(acopy) _whispersounds _returnvalue_3))
  ;[1 1 1] Assign a random sound on pick up and on each clip end choose another random sound from the array as long as it is not the same as the previous one
  (if (not (Variables|Default|GetIsTurnedIn))
    (while (Utilities|Enum|Equal(Enum) (Utilities|GetDisplayName _output) (Utilities|GetDisplayName (Variables|/Script/Engine.AudioComponent|GetSound (Variables|Default|GetWhisperSound))))
      _)
    (Audio|Components|Audio|SetSound (Variables|Default|GetWhisperSound) _output)
    (Utilities|FlowControl|Delay 0.2)
    (Audio|Components|Audio|Play (Variables|Default|GetWhisperSound) 0.0)))

(event EventOnTurnin
  (params (Lantern :type Actor%20Object%20Reference))
  (bind _timetodestroy (Variables|Default|GetTimeToDestroy))
  (Variables|Default|SetLantern Lantern)
  (Variables|Default|SetIsTurnedIn true)
  (Utilities|FlowControl|Sequence
    (:then_0
      (Game|Feedback|ClientPlayForceFeedback (Game|GetPlayerController 0) "/Game/Blueprints/ForceFeedback/ForceFeedbackEffect.ForceFeedbackEffect" "None" false false false)
      (bind _alpha (Timeline|LowerTheScale PlayFromStart)
        (:Update
          (Transformation|SetActorScale3D (* (Variables|Default|GetOriginScale) _alpha)))))
    (:then_1
      (Audio|Components|Audio|FadeOut (Variables|Default|GetWhisperSound) 1.0 0.0 "Linear" :!class /Script/Engine.AudioComponent)
      (Utilities|FlowControl|Delay _timetodestroy)
      (Actor|DestroyActor))
    (:then_2
      (bind _returnvalue (AddComponent|AddAudioComponent false))
      (Audio|Components|Audio|FadeOut _returnvalue _timetodestroy 0.0 "Linear" :!class /Script/Engine.AudioComponent))
    (:then_3
      (Audio|PlaySoundatLocation "/Game/Sounds/SFX/Souls/Magic/ESM_Magic_Game_Spell_Whoosh_15_Fantasy_Cast_Craft_Mobile_App_Special_Touch_Pickup_Click.ESM_Magic_Game_Spell_Whoosh_15_Fantasy_Cast_Craft_Mobile_App_Special_Touch_Pickup_Click" (Transformation|GetWorldLocation (Variables|Default|GetCube)) "0, 0, 0" 1.0 1.0 0.0 0 0 0))))

(event EventBeginPlay
  (bind _returnvalue (Transformation|GetActorLocation))
  (Variables|Default|SetStartLocation (Transformation|GetActorLocation))
  (bind _newtrack_0 (Timeline|Timeline_0 PlayFromStart)
    (:Update
      (Transformation|SetActorLocation (Math|Vector|MakeVector (.x _returnvalue) (.y _returnvalue) (.z (+ (Math|Vector|MakeVector 0.0 0.0 _newtrack_0) (Transformation|GetActorLocation)))) false false))
    (:Finished
      (if true
        (Timeline|Timeline_0 ReverseFromEnd)))))

(event EventTick
  (params (DeltaSeconds :type Float%20%28single-precision%29))
  (bind _lantern (Variables|Default|GetLantern))
  (bind _returnvalue (Utilities|SoulMovement _lantern))
  (if (Variables|Default|GetIsTurnedIn)
    (Transformation|SetActorLocation (Math|Vector|MakeVector (.x _returnvalue) (.y _returnvalue) (+ (.z _returnvalue) (Variables|Default|GetLamternTurnInOffset))) false false)
    (Utilities|FlowControl|DoOnce false
      (:Completed
        (Class|ITeleporterInterface|LastSoulTurnedin (Variables|SoulActor|Gettelie))))
    (else
      (Utilities|FlowControl|Sequence
        (:then_0
          (bind _pawntofollow (Variables|Default|GetPawnToFollow)
            (:then
              (if (< (Variables|Default|GetDistanceBehindPawn) (Math|Vector|Distance(Vector) (Transformation|GetActorLocation) (Transformation|GetActorLocation _pawntofollow)))
                (Transformation|SetActorLocation (Utilities|SoulMovement (Variables|Default|GetPawnToFollow)) false false)))
            (:else)))))))

(event EventOnPickedUp
  (params (Pawn :type Pawn%20Object%20Reference))
  (bind _whispersounds (Variables|Default|GetWhisperSounds))
  (bind _returnvalue (Utilities|Array|Length _whispersounds))
  (bind _returnvalue_2 (- _returnvalue 1))
  (bind _returnvalue_3 (Math|Random|RandomInteger _returnvalue_2))
  (bind _output (Utilities|Array|Get(acopy) _whispersounds _returnvalue_3))
  (Utilities|FlowControl|Sequence
    (:then_0
      (bind _asteam_09_dark_light_character (Utilities|Casting|CastToTeam09_DarkLightCharacter Pawn))
      (Variables|Default|SetPlaceInLine (+ (Utilities|Array|Length (Variables|/Script/Team09_DarkLight.Team09_DarkLightCharacter|GetHeldSouls _asteam_09_dark_light_character)) 1))
      (Variables|Default|SetPawnToFollow _asteam_09_dark_light_character)
      (Actor|Tick|SetActorTickEnabled true)
      (Collision|SetCollisionEnabled (Variables|Default|GetBoxComponent) "NoCollision")
      (Collision|SetCollisionEnabled (Variables|Default|GetBoxComponent) "NoCollision")
      (Variables|Default|SetIsTurnedIn false)
      (Utilities|FlowControl|Sequence
        (:then_0
          (Class|LightComponent|SetIESBrightnessScale (Variables|Default|GetLightUp) 6e+03)
          (Variables|Default|SetOriginScale (Transformation|GetActorScale3D) :!label _label)
          (bind _alpha (Timeline|ScaleFeedback Play)
            (:Update
              (Transformation|SetActorScale3D (Math|Vector|Lerp(Vector) (Variables|Default|GetOriginScale) (* (Variables|Default|GetOriginScale) 1.5) _alpha)))))
        (:then_1
          (Class|LightComponent|SetIESBrightnessScale (Variables|Default|GetLightDown) 2.5e+05))
        (:then_2
          (goto _label))))
    (:then_1
      ;[1 1 1] Assign a random sound on pick up and on each clip end choose another random sound from the array as long as it is not the same as the previous one
      (bind _returnvalue_4 (AddComponent|AddAudioComponent false))
      (Variables|Default|SetWhisperSound _returnvalue_4)
      (while (== _output (Variables|/Script/Engine.AudioComponent|GetSound (Variables|Default|GetWhisperSound)))
        _)
      (Audio|Components|Audio|SetSound (Variables|Default|GetWhisperSound) _output)
      (EventDispatchers|AssignOnAudioFinished (Variables|Default|GetWhisperSound) (delegate Custom|OnAudioFinished_Event_0)))
    (:then_2
      (Game|Feedback|ClientPlayForceFeedback (Game|GetPlayerController 0) "/Game/Blueprints/ForceFeedback/ForceFeedbackEffect.ForceFeedbackEffect" "None" false false false))))

(fn ConstructionScript)