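; Breakable bottle prop built on a destructible mesh component, with sound feedback for impacts and breakage.
; A component hit plays a glass clink at the mesh location, throttled by a DoOnce that resets after a short delay to avoid repeated sounds.
; Fracturing plays a glass crash sound there, then destroys the actor after a few seconds.
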(event OnComponentFracture(SM_Prop_bottle_01_DM)
  (params (HitPoint :type Vector%20%28by%20ref%29 :default "0, 0, 0") (HitDirection :type Vector%20%28by%20ref%29 :default "0, 0, 0"))
  (Audio|PlaySoundatLocation "/Game/Sounds/SFX/Glass/CrashGlassVase_S08IM_117.CrashGlassVase_S08IM_117" (Transformation|GetWorldLocation (Variables|Default|GetSM_Prop_bottle_01_DM)) "0, 0, 0" 1.0 1.0 0.0 0 0 0)
  (Utilities|FlowControl|Delay 5.0)
  (Actor|DestroyActor))

(event OnComponentHit(SM_Prop_bottle_01_DM)
  (params (HitComponent :type Primitive%20Component%20Object%20Reference) (OtherActor :type Actor%20Object%20Reference) (OtherComp :type Primitive%20Component%20Object%20Reference) (NormalImpulse :type Vector :default "0, 0, 0") (Hit :type Hit%20Result%20Structure%20%28by%20ref%29))
  (Utilities|FlowControl|DoOnce false :!label _label
    (:Completed
      (Audio|PlaySoundatLocation "/Game/Sounds/SFX/Glass/Soundiron_Crystal_Glass_56.Soundiron_Crystal_Glass_56" (Transformation|GetWorldLocation (Variables|Default|GetSM_Prop_bottle_01_DM)) "0, 0, 0" 1.0 1.0 0.0 0 0 0)
      (Utilities|FlowControl|Delay 0.5)
      (goto _label Reset))))

(event EventBeginPlay)

(event Collision|EventActorBeginOverlap
  (params (OtherActor :type Actor%20Object%20Reference)))

(event EventTick
  (params (DeltaSeconds :type Float%20%28single-precision%29)))

(fn ConstructionScript)