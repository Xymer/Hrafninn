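; Base actor for objects that belong to one realm, visible and solid only while that realm is current.
; On BeginPlay it caches GameMode_GamePlay, binds to OnRealmSwap and hides its Object component if its Realm differs from CurrentRealm.
; Each swap re-compares the two and toggles visibility and collision to match.
; Older debug and toggle logic remains in the graph unconnected.
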(event Custom|OnRealmSwap_Event
  (bind _object (Variables|Default|GetObject))
  (bind _object_2 (Variables|Default|GetObject))
  (if (Utilities|Enum|Equal(Enum) (Variables|Default|GetRealm) (Variables|/Game/SideScrollerCPP/Core/GameMode_GamePlay.GameMode_GamePlay_C|GetCurrentRealm (Variables|Default|GetCurrentGameMode)))
    (Rendering|SetVisibility _object_2 true false)
    (Collision|SetCollisionEnabled _object_2 "QueryAndPhysics")
    (else
      (Rendering|SetVisibility _object false false)
      (Collision|SetCollisionEnabled _object "NoCollision"))))

(event EventBeginPlay
  (bind _object (Variables|Default|GetObject))
  (bind _asgame_mode_game_play (Utilities|Casting|CastToGameMode_GamePlay (Game|GetGameMode)))
  (Variables|Default|SetCurrentGameMode _asgame_mode_game_play)
  (EventDispatchers|BindEventtoOnRealmSwap (delegate Custom|OnRealmSwap_Event))
  (Input|EnableInput (Game|GetPlayerController 0))
  (if (not (Utilities|Enum|Equal(Enum) (Variables|Default|GetRealm) (Variables|/Game/SideScrollerCPP/Core/GameMode_GamePlay.GameMode_GamePlay_C|GetCurrentRealm (Variables|Default|GetCurrentGameMode))))
    (Rendering|SetVisibility _object false false)
    (Collision|SetCollisionEnabled _object "NoCollision")))

(event Collision|EventActorBeginOverlap
  (params (OtherActor :type Actor%20Object%20Reference)))

(event EventTick
  (params (DeltaSeconds :type Float%20%28single-precision%29)))

(fn ConstructionScript)