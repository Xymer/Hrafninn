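; BP_Gate is a prototype gate that opens on OnOpen and shuts behind the player.
; The OpenDoorLine timeline slides the actor vertically from the height cached at BeginPlay.
; When the player character overlaps CloseTrigger, the timeline reverses and the initially disabled InvisibleWall collision turns on.
; OnClose is empty, and a duplicate Timeline_0 movement graph never runs.
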(event OnComponentBeginOverlap(CloseTrigger)
  (params (OverlappedComponent :type Primitive%20Component%20Object%20Reference) (OtherActor :type Actor%20Object%20Reference) (OtherComp :type Primitive%20Component%20Object%20Reference) (OtherBodyIndex :type Integer) (bFromSweep :type Boolean) (SweepResult :type Hit%20Result%20Structure%20%28by%20ref%29))
  (bind _returnvalue (Transformation|GetActorLocation))
  (Utilities|Casting|CastToTeam09_DarkLightCharacter OtherActor)
  (Collision|SetCollisionEnabled (Variables|Default|GetInvisibleWall) "QueryAndPhysics")
  (bind _openclosetime (Timeline|OpenDoorLine Reverse)
    (:Update
      (Transformation|SetActorLocation (Math|Vector|MakeVector (.x _returnvalue) (.y _returnvalue) (- (Variables|Default|GetStartingHeight) (* _openclosetime -2e+02))) false false))))

(event EventBeginPlay
  (Variables|Default|SetStartingHeight (.z (Transformation|GetActorLocation)))
  (Collision|SetCollisionEnabled (Variables|Default|GetInvisibleWall) "NoCollision"))

(event Collision|EventActorBeginOverlap
  (params (OtherActor :type Actor%20Object%20Reference)))

(event EventTick
  (params (DeltaSeconds :type Float%20%28single-precision%29)))

(event EventOnOpen
  (bind _returnvalue (Transformation|GetActorLocation))
  (bind _openclosetime (Timeline|OpenDoorLine Play)
    (:Update
      (Transformation|SetActorLocation (Math|Vector|MakeVector (.x _returnvalue) (.y _returnvalue) (- (Variables|Default|GetStartingHeight) (* _openclosetime -2e+02))) false false))))

(event EventOnClose)

(fn ConstructionScript)