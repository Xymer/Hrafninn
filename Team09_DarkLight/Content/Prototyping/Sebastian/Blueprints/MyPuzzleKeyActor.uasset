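; Puzzle key actor that, once picked up by the DarkLight character, trails that pawn as a held key.
; Pickup sets its place in line from the held key count, enables Tick and disables collision.
; Tick moves it via SoulMovement beyond a distance threshold, showing its light, and drives a ping-pong Hover timeline.
; SoulMovement contains a distance-scaled lerp toward a queue-offset position, shown as unused.
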(event EventBeginPlay)

(event Collision|EventActorBeginOverlap
  (params (OtherActor :type Actor%20Object%20Reference)))

(event EventTick
  (params (DeltaSeconds :type Float%20%28single-precision%29))
  (Utilities|FlowControl|Sequence
    (:then_0
      (bind _pawntofollow (Variables|Default|GetPawnToFollow)
        (:then
          (if (< 6e+01 (Math|Vector|Distance(Vector) (Transformation|GetActorLocation) (Transformation|GetActorLocation _pawntofollow)))
            (Transformation|SetActorLocation (Utilities|SoulMovement) false false)
            (Rendering|SetVisibility (Variables|Default|GetPointLight) true false)))
        (:else)))
    (:then_1
      (bind _hovertrack (Timeline|Hover Play)
        (:Update
          (Transformation|SetActorLocation (+ (Math|Vector|MakeVector 0.0 0.0 _hovertrack) (Transformation|GetActorLocation)) false false))
        (:Finished
          (if true
            (Timeline|Hover ReverseFromEnd)))))))

(event EventOnPickedUp
  (params (Pawn :type Pawn%20Object%20Reference))
  (bind _asteam_09_dark_light_character (Utilities|Casting|CastToTeam09_DarkLightCharacter Pawn))
  (Variables|Default|SetPlaceInLine (+ (Utilities|Array|Length (Variables|/Script/Team09_DarkLight.Team09_DarkLightCharacter|GetHeldKeys _asteam_09_dark_light_character)) 1))
  (Variables|Default|SetPawnToFollow _asteam_09_dark_light_character)
  (Actor|Tick|SetActorTickEnabled true)
  (Collision|SetCollisionEnabled (Variables|Default|GetCube) "NoCollision")
  (Collision|SetCollisionEnabled (Variables|Default|GetBoxComponent) "NoCollision"))

(fn ConstructionScript)