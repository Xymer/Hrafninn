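; Prototype soul actor that bobs in place and flies toward the player when approached.
; A self-calling Move event chains latent MoveComponentTo calls to loop the static mesh's height and yaw animation from BeginPlay.
; When an actor implementing BPI_Soul overlaps the box, the root component moves to player character 0's location.
; The file contains no pickup or destroy logic.
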(event OnComponentBeginOverlap(Box)
  (params (OverlappedComponent :type Primitive%20Component%20Object%20Reference) (OtherActor :type Actor%20Object%20Reference) (OtherComp :type Primitive%20Component%20Object%20Reference) (OtherBodyIndex :type Integer) (bFromSweep :type Boolean) (SweepResult :type Hit%20Result%20Structure%20%28by%20ref%29))
  (if (Utilities|DoesObjectImplementInterface OtherActor "/Game/Prototyping/Artur/Blueprints/Interface/BPI_Soul.BPI_Soul_C")
    (Components|MoveComponentTo (Variables|Default|GetDefaultSceneRoot) (Transformation|GetWorldLocation (Variables|/Script/Engine.Actor|GetRootComponent (Game|GetPlayerCharacter 0))) "0, 0, 0" false false 0.5 false)))

(event Custom|Move
  (Components|MoveComponentTo (Variables|Default|GetStaticMesh) (Math|Vector|MakeVector 0.0 0.0 125.0) (Math|Rotator|MakeRotator 0.0 0.0 1.8e+02) false false 1.0 false)
  (Components|MoveComponentTo (Variables|Default|GetStaticMesh) (Math|Vector|MakeVector 0.0 0.0 115.0) (Math|Rotator|MakeRotator 0.0 0.0 0.0) false false 1.0 false)
  (CallFunction|Move))

(event EventBeginPlay
  (CallFunction|Move))

(fn ConstructionScript)